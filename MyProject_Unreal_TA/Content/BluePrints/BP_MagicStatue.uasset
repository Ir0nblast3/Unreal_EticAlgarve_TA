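; Interactable statue actor that sends the player on to another level.
; Overlapping its collision enables interaction and shows an E prompt widget, which is removed when the overlap ends.
; On BeginPlay it binds to the player controller's E-press event to drive interaction.
; Interacting finds the current level in the Levels array and opens the hardcoded level at the following index.
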(event `self.StatueInteractableCollisiom.OnComponentBeginOverlap`
  (params (OverlappedComponent :type "PrimitiveComponent Object Reference") (OtherActor :type "Actor Object Reference") (OtherComp :type "PrimitiveComponent Object Reference") (OtherBodyIndex :type Integer) (bFromSweep :type Boolean) (SweepResult :type "HitResult Structure (by ref)"))
  (set `self.CanInteract` true)
  (bind _returnvalue (`|CreateWidget` "/Game/Widgets/E_Widget_TA.E_Widget_TA_C"))
  (bind _output_get (set `self.NewVar` _returnvalue))
  (`UserWidget.AddToViewport` _output_get 0))

(event `self.ReceiveBeginPlay`
  (bind _asplayer_controller_ta (cast `/Game/BluePrints/PlayerControllerTA` (`GameplayStatics.GetPlayerController` 0)))
  (add `/Game/BluePrints/PlayerControllerTA.OnEPressed` _asplayer_controller_ta (`|CreateDelegate` :!event `Interact`)))

(event `self.StatueInteractableCollisiom.OnComponentEndOverlap`
  (params (OverlappedComponent :type "PrimitiveComponent Object Reference") (OtherActor :type "Actor Object Reference") (OtherComp :type "PrimitiveComponent Object Reference") (OtherBodyIndex :type Integer))
  (set `self.CanInteract` false)
  (`Widget.RemoveFromParent` (`self.NewVar`)))

(event `Interact`
  (if (`self.CanInteract`)
    (`KismetSystemLibrary.PrintString` "Hello")
    (bind _returnvalue (`GameplayStatics.GetCurrentLevelName` true))
    (`GameplayStatics.OpenLevel` (select `int` (+ (`KismetArrayLibrary.Array_Find` (`self.Levels`) (`KismetStringLibrary.Conv_StringToName` _returnvalue)) 1) :`0` "Minimal_Default" :`1` "Nivel2" :`2` "Nivel3" :!type "Name"))))

(fn `UserConstructionScript`)