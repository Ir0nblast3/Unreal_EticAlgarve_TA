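; BP_FallingPlatform is a platform actor that repeatedly tilts on its pitch axis and back, with no trigger or player interaction.
; After a variable start delay on BeginPlay, one timeline drives the pitch while preserving roll and yaw.
; A second timeline then plays in reverse from its end, and the two alternate indefinitely with a fixed pause between swings.
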(event `self.ReceiveBeginPlay`
  (`KismetSystemLibrary.Delay` (`self.Time`))
  (bind (_direction _rotation) (`Timeline|Timeline` :!label _label)
    (:`Update`
      (`self.K2_SetActorRotation` (`KismetMathLibrary.MakeRotator` (.roll (`self.K2_GetActorRotation`)) _rotation (.yaw (`self.K2_GetActorRotation`)))))
    (:`Finished`
      (`KismetSystemLibrary.Delay` 2.0)
      (bind (_direction_2 _rotation_2) (`Timeline|Timeline_0` :!via `ReverseFromEnd`)
        (:`Update`
          (`self.K2_SetActorRotation` (`KismetMathLibrary.MakeRotator` (.roll (`self.K2_GetActorRotation`)) _rotation_2 (.yaw (`self.K2_GetActorRotation`)))))
        (:`Finished`
          (`KismetSystemLibrary.Delay` 2.0)
          (goto _label :!via `PlayFromStart`))))))

(fn `UserConstructionScript`)