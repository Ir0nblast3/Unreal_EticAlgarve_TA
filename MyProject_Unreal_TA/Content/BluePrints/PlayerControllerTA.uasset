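; Player controller that shows the game over, pause and win screens.
; On BeginPlay it casts the player character to BP_ThirdPersonCharacter and binds to the OnGameOver dispatcher on its health component.
; Its death, pause and win events each create their widget, add it to the viewport, switch input to UI only and show the mouse cursor.
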(event `self.ReceiveBeginPlay`
  (`parent.ReceiveBeginPlay`)
  (bind _asbp_third_person_character (cast `/Game/ThirdPerson/Blueprints/BP_ThirdPersonCharacter` (`GameplayStatics.GetPlayerCharacter` 0)))
  (add `/Game/BluePrints/BP_HealthComponent.OnGameOver` (`/Game/ThirdPerson/Blueprints/BP_ThirdPersonCharacter.BP_HealthComponent` _asbp_third_person_character) (`|CreateDelegate` :!event `OnPlayerDead`)))

(event `OnPlayerDead`
  (bind _returnvalue (`|CreateWidget` "/Game/Widgets/W_GameOver.W_GameOver_C"))
  (`UserWidget.AddToViewport` _returnvalue 0)
  (`WidgetBlueprintLibrary.SetInputMode_UIOnlyEx` self _returnvalue)
  (set `self.bShowMouseCursor` true))

(event `OnPause`
  (bind _returnvalue (`|CreateWidget` "/Game/Widgets/W_PauseMenu.W_PauseMenu_C"))
  (`UserWidget.AddToViewport` _returnvalue 0)
  (`WidgetBlueprintLibrary.SetInputMode_UIOnlyEx` self _returnvalue)
  (set `self.bShowMouseCursor` true))

(event `GameWon`
  (bind _returnvalue (`|CreateWidget` "/Game/Widgets/W_WonGame.W_WonGame_C"))
  (`UserWidget.AddToViewport` _returnvalue 0)
  (`WidgetBlueprintLibrary.SetInputMode_UIOnlyEx` self _returnvalue)
  (set `self.bShowMouseCursor` true))

(fn `UserConstructionScript`)