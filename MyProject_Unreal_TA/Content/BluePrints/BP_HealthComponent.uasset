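; Health component that stores a health value and signals when it changes or runs out.
; On BeginPlay it binds a handler to OnHealthChange, which adds the passed amount to Health and clamps the result between 0 and 100.
; Each change calls UpdateProgressBar, and reaching zero also calls OnGameOver.
; GetHealth exposes the current value.
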(event `self.ReceiveBeginPlay`
  (add `self.OnHealthChange` (`|CreateDelegate` :!event `CustomEvent`)))

(event `CustomEvent` :!signature `self.OnHealthChange`
  (params (NewParam :type "Float (double-precision)"))
  (bind _output_get (set `self.Health` (+ NewParam (`self.Health`))))
  (bind _output_get_2 (set `self.Health` (`KismetMathLibrary.FClamp` _output_get 0.0 100.0)))
  (`self.UpdateProgressBar`)
  (if (<= _output_get_2 0.0)
    (`self.OnGameOver`)))

(fn `BP_HealthComponent_AutoGenFunc`)

(fn `GetHealth`
  (returns (Health :type "Float (double-precision)"))
  (return (`self.Health`)))