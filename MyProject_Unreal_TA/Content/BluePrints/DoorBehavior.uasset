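; Interactable door Blueprint that swings its static mesh open and closed when the player is within range.
; A collision overlap sets CanInteract and shows or removes an E prompt widget.
; BeginPlay binds to the player controller's E-press dispatcher, and the Interact event plays a timeline forward or in reverse based on IsDoorOpen.
; The timeline drives the mesh's relative yaw and flips the open state when finished.
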(event `self.DoorInteractableColision.OnComponentEndOverlap`
  (params (OverlappedComponent :type "PrimitiveComponent Object Reference") (OtherActor :type "Actor Object Reference") (OtherComp :type "PrimitiveComponent Object Reference") (OtherBodyIndex :type Integer))
  (set `self.CanInteract` false)
  (`Widget.RemoveFromParent` (`self.Widget`)))

(event `self.ReceiveBeginPlay`
  (bind _asplayer_controller_ta (cast `/Game/BluePrints/PlayerControllerTA` (`GameplayStatics.GetPlayerController` 0)))
  (add `/Game/BluePrints/PlayerControllerTA.OnEPressed` _asplayer_controller_ta (`|CreateDelegate` :!event `Interact`)))

(event `self.DoorInteractableColision.OnComponentBeginOverlap`
  (params (OverlappedComponent :type "PrimitiveComponent Object Reference") (OtherActor :type "Actor Object Reference") (OtherComp :type "PrimitiveComponent Object Reference") (OtherBodyIndex :type Integer) (bFromSweep :type Boolean) (SweepResult :type "HitResult Structure (by ref)"))
  (set `self.CanInteract` true)
  (bind _returnvalue (`|CreateWidget` "/Game/Widgets/E_Widget_TA.E_Widget_TA_C"))
  (bind _output_get (set `self.Widget` _returnvalue))
  (`UserWidget.AddToViewport` _output_get 0))

(event `/Game/BluePrints/BP_Interface_TA.Interact`
  (if (`self.CanInteract`)
    (if (`self.IsDoorOpen`)
      (bind (_direction _dooropening) (`Timeline|My Timeline` :!via `ReverseFromEnd` :!label _label)
        (:`Update`
          (`SceneComponent.K2_SetRelativeRotation` (`self.StaticMesh`) (`KismetMathLibrary.MakeRotator` (.roll (`self.K2_GetActorRotation`)) (.pitch (`self.K2_GetActorRotation`)) _dooropening) false false))
        (:`Finished`
          (set `self.IsDoorOpen` (not (`self.IsDoorOpen`)))))
      (else
        (goto _label :!via `PlayFromStart`)))))

(fn `UserConstructionScript`)